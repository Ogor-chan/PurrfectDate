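; BP_BendedSplineObject is an actor that bends copies of a mesh along its spline at construction time.
; The construction script derives a count from spline length over mesh X-size plus Offset, then adds and attaches a spline mesh component per index.
; Each segment spans consecutive spline points using their local tangents, not distance steps, and its start X is multiplied by Offset.
; The collision-enabling node is unconnected, and the event graph is empty.
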(event EventBeginPlay)

(event Collision|EventActorBeginOverlap
  (params (OtherActor :type Actor%20Object%20Reference)))

(event EventTick
  (params (DeltaSeconds :type Float%20%28single-precision%29)))

(fn ConstructionScript
  (bind _bendedsplinemesh (Variables|Default|GetBendedSplineMesh))
  (bind _spline (Variables|Default|GetSpline))
  (bind _returnvalue (StaticMesh|GetBoundingBox _bendedsplinemesh))
  (bind (_min _max) (Utilities|Struct|BreakBox _returnvalue))
  (bind _output_get (Variables|Default|SetSpacing (+ (.X (Math|Vector|BreakVector (- _max _min))) (Variables|Default|GetOffset))))
  (bind _output_get_2 (LocalVariables|SetNumberOfInstances (Math|Float|Floor (/ (Spline|GetSplineLength (Variables|Default|GetSpline)) _output_get))))
  (for _index (range 0 _output_get_2)
    (bind _returnvalue_2 (AddComponent|AddSplineMeshComponent false))
    (Components|StaticMesh|SetStaticMesh _returnvalue_2 (Variables|Default|GetBendedSplineMesh))
    (SplineMesh|SetStartandEnd _returnvalue_2 (Math|Vector|MakeVector (* (.x (.Location (Spline|GetLocationandTangentatSplinePoint _spline _index "Local"))) (Variables|Default|GetOffset)) (.y (.Location (Spline|GetLocationandTangentatSplinePoint _spline _index "Local"))) (.z (.Location (Spline|GetLocationandTangentatSplinePoint _spline _index "Local")))) (.Tangent (Spline|GetLocationandTangentatSplinePoint _spline _index "Local")) (.Location (Spline|GetLocationandTangentatSplinePoint _spline (+ _index 1) "Local")) (.Tangent (Spline|GetLocationandTangentatSplinePoint _spline (+ _index 1) "Local")) true :!class /Script/Engine.SplineMeshComponent)
    (Transformation|AttachComponentToComponent _returnvalue_2 (Variables|Default|GetDefaultSceneRoot) "None" "KeepRelative" "KeepRelative" "KeepRelative" true)))