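; BastetBP is a touch/click Blueprint in the visual novel framework that selects which Bastet scene to use.
; PickLocalScene checks entry 2 of GlobalBP's MasterChoiceLog, returning BastetScene when it is zero and RepeatBastetScene otherwise.
; Both results leave the travel prompt and breakdown skip flags off.
; The event graph holds only disabled default events, and the construction script just calls its parent.
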(event EventBeginPlay
  (|CallParentFunction) ; This node is disabled and will not be called.\nDrag off pins to build functionality.
)

(event Collision|EventActorBeginOverlap
  (params (OtherActor :type Actor%20Object%20Reference))
  (|CallParentFunction OtherActor) ; This node is disabled and will not be called.\nDrag off pins to build functionality.
)

(event EventTick
  (params (DeltaSeconds :type Float%20%28single-precision%29))
  (|CallParentFunction DeltaSeconds) ; This node is disabled and will not be called.\nDrag off pins to build functionality.
)

(fn ConstructionScript
  (|CallParentFunction))

(fn PickLocalScene
  (if (== (Utilities|Array|Get(acopy) (Variables|/Game/VN_Framework/Blueprints/Global_BP.Global_BP_C|GetMasterChoiceLog (Variables|Default|GetGlobal_BP)) 2) 0)
    (return "BastetScene" false false)
    (else
      (return "RepeatBastetScene" false false))))